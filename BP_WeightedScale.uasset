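; BP_WeightedScale is a puzzle scale that opens a referenced door when the weight on it nearly matches a target, and closes it otherwise.
; Box overlaps add or remove each actor's component mass through a map, updating the clamped total and weight display.
; UpdateStats converts the total to a fraction of maximum weight, drives the door and enables Tick on change.
; Tick eases the scale's height toward that fraction, then disables itself once settled.
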(event OnComponentBeginOverlap(Box)
  (params (OverlappedComponent :type Primitive%20Component%20Object%20Reference) (OtherActor :type Actor%20Object%20Reference) (OtherComp :type Primitive%20Component%20Object%20Reference) (OtherBodyIndex :type Integer) (bFromSweep :type Boolean) (SweepResult :type Hit%20Result%20Structure%20%28by%20ref%29))
  ;[0.15 0.15 0.15 0.5] Function to add or remove objects from the scale, and will update stats to determine z position of the scale
  (CallFunction|ObjectsOff/onScale OtherActor OtherComp true)
  (CallFunction|UpdateStats))

(event OnComponentEndOverlap(Box)
  (params (OverlappedComponent :type Primitive%20Component%20Object%20Reference) (OtherActor :type Actor%20Object%20Reference) (OtherComp :type Primitive%20Component%20Object%20Reference) (OtherBodyIndex :type Integer))
  ;[0.15 0.15 0.15 0.5] Function to add or remove objects from the scale, and will update stats to determine z position of the scale
  (CallFunction|ObjectsOff/onScale OtherActor OtherComp false)
  (CallFunction|UpdateStats))

(event EventBeginPlay)

(event Collision|EventActorBeginOverlap
  (params (OtherActor :type Actor%20Object%20Reference)))

(event EventTick
  (params (DeltaSeconds :type Float%20%28single-precision%29))
  ;[0.15 0.15 0.15 0.5] Optimises game by not having actor tick enabled whilst nothing is happening.
  (if (== (Variables|Default|GetScaleOffsetAmount) (Variables|Default|GetCurrentWeightPercent))
    (Actor|Tick|SetActorTickEnabled false)
    (else
      ;[0.15 0.15 0.15 0.5] Scale will move down depending on the percentage between current weight on scale and the max percentage
      (Variables|Default|SetScaleOffsetAmount (Math|Interpolation|FInterpTo (Variables|Default|GetScaleOffsetAmount) (Variables|Default|GetCurrentWeightPercent) (Utilities|Time|GetWorldDeltaSeconds) 1e+01))
      (Variables|Default|SetScalePosition (Math|Vector|MakeVector 0.0 0.0 (Math|Float|Lerp 1e+02 -5e+01 (Variables|Default|GetScaleOffsetAmount))))
      (Transformation|SetRelativeLocation (Variables|Default|GetScale) (Variables|Default|GetScalePosition) false false))))

(fn ConstructionScript)

(fn ObjectsOff/onScale
  (params (In%20actor :type Actor%20Object%20Reference) (In%20comp :type Primitive%20Component%20Object%20Reference) (Adding? :type Boolean))
  (bind _objectweightmap (Variables|Default|GetObjectWeightMap))
  (bind _value (Utilities|Map|Find _objectweightmap In%20actor))
  (if Adding?
    ;[0.15 0.15 0.15 0.5] Will map the new actor to its mass
    (Utilities|Map|Add (Variables|Default|GetObjectWeightMap) In%20actor (Physics|GetMass In%20comp)))
  (if (Utilities|Map|IsEmpty (Variables|Default|GetObjectWeightMap))
    (bind _output_get (Variables|Default|SetCurrentWeight 0.0))
    (Rendering|Components|TextRender|SetText (Variables|Default|GetWeightDisplay) (Utilities|Text|ToText(Float) _output_get "HalfToEven"))
    (else
      (bind _output_get_2 (Variables|Default|SetCurrentWeight (Math|Float|Clamp(Float) (+ (Variables|Default|GetCurrentWeight) (select Adding? _value (* _value -1.0))) 0.0 (Variables|Default|GetMaxWeight))))
      (Rendering|Components|TextRender|SetText (Variables|Default|GetWeightDisplay) (Utilities|Text|ToText(Float) _output_get_2 "HalfToEven"))))
  ;[0.15 0.15 0.15 0.5] If adding is false, actor has left scales so remove from the map
  (if (not Adding?)
    (Utilities|Map|Remove (Variables|Default|GetObjectWeightMap) In%20actor)))

(fn UpdateStats
  (bind _maxweight (Variables|Default|GetMaxWeight))
  (bind _currentweight (Variables|Default|GetCurrentWeight))
  (bind _returnvalue (/ _currentweight _maxweight))
  (bind _returnvalue_2 (Math|Float|Clamp(Float) _returnvalue))
  ;[0.15 0.15 0.15 0.5] Finds the percentage weight the scale is holding compared to its max weight (used to push down scale depending on the mass)
  (if (not (== (Variables|Default|GetCurrentWeightPercent) _returnvalue_2))
    (Variables|Default|SetCurrentWeightPercent _returnvalue_2)
    ;[0.15 0.15 0.15 0.5] If the current weight is equal to target weight, open the door, otherwise close the door
    (if (Math|Float|NearlyEqual(Float) (Variables|Default|GetCurrentWeight) (Variables|Default|GetTargetWeight) 0.1)
      (Default|DoorOpen (Variables|Default|GetDoorRef))
      (else
        (Default|DoorClose (Variables|Default|GetDoorRef))))
    (Actor|Tick|SetActorTickEnabled true)))